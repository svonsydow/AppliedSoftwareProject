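; BPC_DamageSystem is an actor component that manages health, healing, damage and death.
; TakeDamage takes a damage info struct and uses the CanBeDamaged macro to branch into block, damage or no damage, based on death, invincibility and blocking.
; Event dispatchers announce blocks with parry eligibility, death, and damage responses, which fire only when interruptible or force-interrupted.
; Heal adds health clamped to the maximum while not dead.
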(event EventBeginPlay)

(event EventTick
  (params (DeltaSeconds :type Float%20%28single-precision%29)))

(fn Heal
  (params (HealAmount :type Float%20%28double-precision%29))
  (if (not (Variables|Default|GetIsDead))
    (bind _output_get (Variables|Default|SetHealth (Math|Float|Clamp(Float) (+ HealAmount (Variables|Default|GetHealth)) 0.0 (Variables|Default|GetMaxHealth))))
    (return _output_get)))

(fn TakeDamage
  (params (DamageInfo :type S%20Damage%20Info%20Structure))
  (bind (_damageamount _damagetype _damageresponse _shoulddamageinvincible _canbeblocked _canbeparried _shouldforceinterrupt) (Utilities|Struct|BreakS_DamageInfo DamageInfo))
  (Utilities|CanbeDamaged _shoulddamageinvincible _canbeblocked
    (:BlockDamage
      (Default|CallOnBlocked _canbeparried)
      (return false))
    (:DoDamage
      (bind _output_get (Variables|Default|SetHealth (- (Variables|Default|GetHealth) _damageamount)))
      (if (<= _output_get 0.0)
        (Variables|Default|SetIsDead true)
        (Default|CallOnDeath)
        (return true)
        (elif (or (Variables|Default|GetIsInterruptible) _shouldforceinterrupt)
          (Default|CallOnDamageResponse _damageresponse)
          (return true))))
    (:NoDamage
      (return false))))