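; CharacterSwap is a controller Blueprint that lets the player cycle possession between the TopDownCharacterParent characters in the level.
; On BeginPlay it gathers all those characters into an array and records the player's current character.
; Pressing Q calls NextCharacter, which finds the current character's index, steps to the next or wraps to the first, then possesses that character.
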(event EventBeginPlay
  (bind _outactors (Actor|GetAllActorsOfClass "/Game/Capstone/Blueprints/TopDownCharacterParent.TopDownCharacterParent_C"))
  (Variables|Default|SetCharacters _outactors)
  (bind _astop_down_character_parent (Utilities|Casting|CastToTopDownCharacterParent (Game|GetPlayerCharacter 0)))
  (Variables|Default|SetCurrentCharacter _astop_down_character_parent))

(event EventTick
  (params (DeltaSeconds :type Float%20%28single-precision%29)))

(event Input|KeyboardEvents|Q
  (params (Key :type Key%20Structure :default "None"))
  (:Pressed
    (CallFunction|NextCharacter)))

(fn ConstructionScript)

(fn NextCharacter
  (LocalVariables|SetLocal_Index (Utilities|Array|FindItem (Variables|Default|GetCharacters) (Variables|Default|GetCurrentCharacter)))
  (bind _output_get (LocalVariables|SetLocal_Index (Math|Integer|SelectInt (+ (Utilities|Array|FindItem (Variables|Default|GetCharacters) (Variables|Default|GetCurrentCharacter)) 1) 0 (Utilities|Array|IsValidIndex (Variables|Default|GetCharacters) (+ (Utilities|Array|FindItem (Variables|Default|GetCharacters) (Variables|Default|GetCurrentCharacter)) 1)))))
  (bind _output_get_2 (Variables|Default|SetCurrentCharacter (Utilities|Array|Get(acopy) (Variables|Default|GetCharacters) _output_get)))
  (Pawn|Possess _output_get_2))